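; AvatarController is a controller Blueprint that toggles and reverses the rotation of every Avatar actor in the level.
; Pressing S flips IsRotate on all Avatars.
; Each Tick, it negates a rotating Avatar's RunSpeed when CooldownTimer reaches half a second or CurrentAngleR exceeds MaxAngle in either direction, then resets the timer.
; All Avatars share that one timer, which advances once per rotating Avatar each frame.
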(event EventTick
  (params (DeltaSeconds :type Float%20%28single-precision%29))
  ;[1 1 1] Rotate Forward or Backward
  (bind _outactors (Actor|GetAllActorsOfClass "/Game/Blueprints/Avatar.Avatar_C"))
  (for _array_element _outactors
    (if (Variables|/Game/Blueprints/Avatar.Avatar_C|GetisRotate _array_element)
      (bind _output_get (Variables|Default|SetcooldownTimer (+ (Utilities|Time|GetWorldDeltaSeconds) (Variables|Default|GetcooldownTimer))))
      (if (not (and (< _output_get 0.5) (and (>= (Math|Float|Absolute(Float) (Variables|/Game/Blueprints/Avatar.Avatar_C|GetcurrentAngleR _array_element)) 0.0) (<= (Math|Float|Absolute(Float) (Variables|/Game/Blueprints/Avatar.Avatar_C|GetcurrentAngleR _array_element)) (Variables|/Game/Blueprints/Avatar.Avatar_C|GetmaxAngle _array_element)))))
        (Variables|Default|SetcooldownTimer 0.0)
        (Variables|/Game/Blueprints/Avatar.Avatar_C|SetrunSpeed _array_element (* (Variables|/Game/Blueprints/Avatar.Avatar_C|GetrunSpeed _array_element) -1))))))

(event Collision|EventActorBeginOverlap
  (params (OtherActor :type Actor%20Object%20Reference)))

(event Input|KeyboardEvents|S
  (params (Key :type Key%20Structure :default "None"))
  ;[1 1 1] Press Butten S to Start or Stop the Rotation
  (:Pressed
    (bind _outactors (Actor|GetAllActorsOfClass "/Game/Blueprints/Avatar.Avatar_C"))
    (for _array_element _outactors
      (Variables|/Game/Blueprints/Avatar.Avatar_C|SetisRotate _array_element (not (Variables|/Game/Blueprints/Avatar.Avatar_C|GetisRotate _array_element))))))

(fn ConstructionScript)