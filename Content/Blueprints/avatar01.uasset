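; Avatar Blueprint that procedurally swings its right and left legs in opposite directions to mimic running.
; Each Tick rotates both leg components in world pitch at RunSpeed scaled by delta time, with RotateBackwardR choosing the direction.
; The flag changes when the sampled pitch passes fixed limits, skipping rotation that frame.
; That pitch comes from the owning actor's rotation rather than the leg's, and is printed for debugging.
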(event EventTick
  (params (DeltaSeconds :type Float%20%28single-precision%29))
  (bind _leftleg (Variables|Components|GetLeftLeg))
  (bind _rightleg (Variables|Default|GetRightLeg))
  (bind _run_speed (Variables|Default|GetRun%20Speed))
  (bind _returnvalue (* DeltaSeconds _run_speed))
  (bind _returnvalue_2 (* _returnvalue -1.0))
  ;[1 1 1] Declare
  (bind _output_get (Variables|Default|SetCurrentAngleR (.Pitch (Math|Rotator|BreakRotator (Transformation|GetActorRotation (Components|GetOwner _rightleg))))))
  (Development|PrintString (Utilities|String|ToString(Float) _output_get))
  (bind _output_get_2 (Variables|Default|SetminAngle -45.0))
  (bind _output_get_3 (Variables|Default|SetmaxAngle 45.0))
  ;[1 1 1] Conditions
  (if (< _output_get _output_get_2)
    (Variables|Default|SetbRotateBackwardR false)
    (elif (> _output_get _output_get_3)
      (Variables|Default|SetbRotateBackwardR true)
      (else
        ;[1 1 1] Run
        (if (Variables|Default|GetbRotateBackwardR)
          (Transformation|AddWorldRotation _rightleg (Math|Rotator|MakeRotator 0.0 _returnvalue 0.0) false false)
          (Transformation|AddWorldRotation _leftleg (Math|Rotator|MakeRotator 0.0 _returnvalue_2 0.0) false false)
          (Variables|Default|SetCurrentAngleR 0.0)
          (else
            (Transformation|AddWorldRotation _rightleg (Math|Rotator|MakeRotator 0.0 _returnvalue_2 0.0) false false)
            (Transformation|AddWorldRotation _leftleg (Math|Rotator|MakeRotator 0.0 _returnvalue 0.0) false false)))))))

(fn ConstructionScript)