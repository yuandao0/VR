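; Avatar Blueprint that animates a simple running motion by rotating its two leg components in code.
; While IsRotate is set, Tick pitches RightLeg and LeftLeg in opposite directions by RunSpeed each frame, without delta-time scaling.
; It also stores the right leg's world pitch in CurrentAngleR.
; When IsRotate is off, it adds zero rotation, so the legs hold their current pose.
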(event EventTick
  (params (DeltaSeconds :type Float%20%28single-precision%29))
  (bind _leftleg (Variables|Components|GetLeftLeg))
  (bind _rightleg (Variables|Default|GetRightLeg))
  (bind _runspeed (Variables|Default|GetrunSpeed))
  (if (Variables|Default|GetisRotate)
    ;[1 1 1] Start Rotation
    (Transformation|AddLocalRotation _rightleg (Math|Rotator|MakeRotator 0.0 (Math|Conversions|ToFloat(Integer) _runspeed) 0.0) false false)
    (Transformation|AddLocalRotation _leftleg (Math|Rotator|MakeRotator 0.0 (Math|Conversions|ToFloat(Integer) (* _runspeed -1)) 0.0) false false)
    ;[1 1 1] Get Current Rotation Angle
    (Variables|Default|SetcurrentAngleR (.Pitch (Math|Rotator|BreakRotator (Transformation|GetWorldRotation _rightleg))))
    (else
      ;[1 1 1] Stop Rotation
      (Transformation|AddLocalRotation _rightleg "0, 0, 0" false false)
      (Transformation|AddLocalRotation _leftleg "0, 0, 0" false false))))

(fn ConstructionScript)