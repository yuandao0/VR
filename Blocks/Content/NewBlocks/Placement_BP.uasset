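; Block placement Blueprint that shows a configurable block mesh and computes a grid-aligned position for it.
; BeginPlay assigns BlockMesh to the Mesh component.
; ReleasePosition line-traces 500 units forward on Visibility from a scene component of the first-person character, with persistent debug drawing.
; On a hit, it returns the impact location snapped to GridSize; nothing here moves or spawns the block.
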(event EventBeginPlay
  (Components|StaticMesh|SetStaticMesh (Variables|Default|GetMesh) (Variables|Default|GetBlock%20Mesh)))

(fn ConstructionScript)

(fn ReleasePosition
  (bind _returnvalue (Actor|GetActorOfClass "/Game/FirstPerson/Blueprints/BP_FirstPersonCharacter.BP_FirstPersonCharacter_C"))
  (bind (_outhit _returnvalue_2) (Collision|LineTraceByChannel (.location (Transformation|GetWorldTransform (Actor|GetComponentbyClass _returnvalue "/Script/Engine.SceneComponent"))) (+ (.location (Transformation|GetWorldTransform (Actor|GetComponentbyClass _returnvalue "/Script/Engine.SceneComponent"))) (* (Math|Vector|GetForwardVector (.rotation (Transformation|GetWorldTransform (Actor|GetComponentbyClass _returnvalue "/Script/Engine.SceneComponent")))) 5e+02)) "TraceTypeQuery1" false 0 "Persistent"))
  (if _returnvalue_2
    (return (Class|KismetMathLibrary|VectorSnappedtoGrid (.Location (Collision|BreakHitResult _outhit)) (Variables|Default|GetGrid%20Size)))))